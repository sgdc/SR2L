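; AssembledArrow is an arrow actor in the advanced vehicle Blueprint content that continuously bobs up and down.
; BeginPlay stores its starting location as the anchor for the motion.
; Tick accumulates a time-scaled angle and sets the height to the starting Z plus a degree-based sine scaled by Range, keeping the original X and Y without sweeping.
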(event `self.ReceiveBeginPlay`
  (set `self.StartingVector` (`self.K2_GetActorLocation`)))

(event `self.ReceiveTick`
  (params (DeltaSeconds :type "Float (single-precision)"))
  (bind _output_get (set `self.SinValue` (+ (* DeltaSeconds 225.0) (`self.SinValue`))))
  (`self.K2_SetActorLocation` (`KismetMathLibrary.MakeVector` (.x (`self.StartingVector`)) (.y (`self.StartingVector`)) (+ (.z (`self.StartingVector`)) (* (`self.Range`) (`KismetMathLibrary.DegSin` _output_get))))))

(fn `UserConstructionScript`)