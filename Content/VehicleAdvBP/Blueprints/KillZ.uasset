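; KillZ is a kill volume actor that respawns the player's vehicle when it overlaps it.
; Unless the vehicle's HUD reports a win, it refills boost, sets a small upward velocity and clears spin.
; It then levels the mesh to the stored spawn yaw and teleports the vehicle slightly above its stored spawn location.
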(event `self.ReceiveActorBeginOverlap`
  (params (OtherActor :type "Actor Object Reference"))
  (bind _asvehicle_blueprint (cast `/Game/VehicleAdvBP/Blueprints/VehicleBlueprint` OtherActor))
  (if (not (`/Game/VehicleAdvBP/Blueprints/BoostHUD.hasWon` (`/Game/VehicleAdvBP/Blueprints/VehicleBlueprint.MyHUD` _asvehicle_blueprint)))
    (set `/Game/VehicleAdvBP/Blueprints/VehicleBlueprint.CurrentBoost` (`/Game/VehicleAdvBP/Blueprints/VehicleBlueprint.BoostMax` _asvehicle_blueprint) _asvehicle_blueprint)
    (bind _mesh (`WheeledVehicle.Mesh` _asvehicle_blueprint))
    (`PrimitiveComponent.SetAllPhysicsLinearVelocity` _mesh (0.0 0.0 500.0) false)
    (`PrimitiveComponent.SetPhysicsAngularVelocity` _mesh (0.0 0.0 0.0) false "None")
    (`SceneComponent.K2_SetWorldRotation` (`WheeledVehicle.Mesh` _asvehicle_blueprint) (`KismetMathLibrary.MakeRotator` 0.0 0.0 (`/Game/VehicleAdvBP/Blueprints/VehicleBlueprint.SpawnYaw` _asvehicle_blueprint)) false false)
    (`self.K2_SetActorLocation` _asvehicle_blueprint (`KismetMathLibrary.MakeVector` (.x (`/Game/VehicleAdvBP/Blueprints/VehicleBlueprint.SpawnLocation` _asvehicle_blueprint)) (.y (`/Game/VehicleAdvBP/Blueprints/VehicleBlueprint.SpawnLocation` _asvehicle_blueprint)) (+ (.z (`/Game/VehicleAdvBP/Blueprints/VehicleBlueprint.SpawnLocation` _asvehicle_blueprint)) 25.0)) false true)))

(fn `UserConstructionScript`)