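; Checkpoint actor that updates a vehicle's respawn point when the vehicle drives into it.
; On actor overlap it casts to VehicleBlueprint and writes that vehicle's SpawnLocation and SpawnYaw from its own transform.
; The spawn position is offset along the checkpoint's local X axis in proportion to the vehicle's ID, giving each vehicle a separate slot.
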(event `self.ReceiveBeginPlay`)

(event `self.ReceiveActorBeginOverlap`
  (params (OtherActor :type "Actor Object Reference"))
  (bind _returnvalue (`self.K2_GetActorRotation`))
  (bind _asvehicle_blueprint (cast `/Game/VehicleAdvBP/Blueprints/VehicleBlueprint` OtherActor))
  (set `/Game/VehicleAdvBP/Blueprints/VehicleBlueprint.SpawnLocation` (+ (`self.K2_GetActorLocation`) (`KismetMathLibrary.GreaterGreater_VectorRotator` (* (`KismetMathLibrary.MakeVector` 75.0) (`/Game/VehicleAdvBP/Blueprints/VehicleBlueprint.ID` _asvehicle_blueprint)) _returnvalue)) _asvehicle_blueprint)
  (set `/Game/VehicleAdvBP/Blueprints/VehicleBlueprint.SpawnYaw` (.yaw _returnvalue) _asvehicle_blueprint))

(event `self.ReceiveTick`
  (params (DeltaSeconds :type "Float (single-precision)")))

(fn `UserConstructionScript`)