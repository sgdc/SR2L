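; Level setup actor that adds a second local player and creates the shared boost HUD for the vehicle game.
; On BeginPlay it spawns the player with a pawn and tags that VehicleBlueprint with its ID.
; It seeds a BoostHUD widget's two boost values from that vehicle's maximum, adds it to the viewport, and hands the same widget to every VehicleBlueprint in the level.
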(event `self.ReceiveBeginPlay`
  (`GameplayStatics.CreatePlayer` 1)
  (bind _asvehicle_blueprint (cast `/Game/VehicleAdvBP/Blueprints/VehicleBlueprint` (`GameplayStatics.GetPlayerPawn` 1)))
  (set `/Game/VehicleAdvBP/Blueprints/VehicleBlueprint.ID` 1 _asvehicle_blueprint)
  (bind _returnvalue (`|CreateWidget` "/Game/VehicleAdvBP/Blueprints/BoostHUD.BoostHUD_C"))
  (bind _output_get (set `/Game/VehicleAdvBP/Blueprints/BoostHUD.BoostMax` (`/Game/VehicleAdvBP/Blueprints/VehicleBlueprint.BoostMax` _asvehicle_blueprint) _returnvalue))
  (bind _output_get_2 (set `/Game/VehicleAdvBP/Blueprints/BoostHUD.BoostCurrent` _output_get _returnvalue))
  (set `/Game/VehicleAdvBP/Blueprints/BoostHUD.BoostCurrent2` _output_get_2 _returnvalue)
  (`UserWidget.AddToViewport` _returnvalue 0)
  (bind _outactors (`GameplayStatics.GetAllActorsOfClass` "/Game/VehicleAdvBP/Blueprints/VehicleBlueprint.VehicleBlueprint_C"))
  (for _array_element _outactors
    (set `/Game/VehicleAdvBP/Blueprints/VehicleBlueprint.MyHUD` _returnvalue _array_element)))

(event `self.ReceiveActorBeginOverlap`
  (params (OtherActor :type "Actor Object Reference")))

(event `self.ReceiveTick`
  (params (DeltaSeconds :type "Float (single-precision)")))

(fn `UserConstructionScript`)